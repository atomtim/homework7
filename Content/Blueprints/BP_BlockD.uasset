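; BP_BlockD is a child Blueprint for a block actor that changes its scale when another actor overlaps it.
; After calling the parent overlap handler, it multiplies Size by K, lowers K by a small uniform step and prints K.
; Following a short delay, it sets the actor scale to K itself, so the computed Size is not applied in this graph.
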(event Collision|EventActorBeginOverlap
  (params (OtherActor :type Actor%20Object%20Reference))
  (|CallParentFunction OtherActor)
  (Variables|Default|SetSize (* (Variables|Default|GetSize) (Variables|Default|GetK)))
  (bind _output_get (Variables|Default|SetK (- (Variables|Default|GetK) "0.050000,0.050000,0.050000")))
  (Development|PrintString (Utilities|String|ToString(Vector) _output_get))
  (Utilities|FlowControl|Delay 0.1)
  (Transformation|SetActorScale3D _output_get))

(fn ConstructionScript
  (|CallParentFunction))